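; BP_IAPawn is the AI player pawn for the red team in a troop-and-tower game with money, experience and ages.
; It caches BP_GameManager on BeginPlay to reach the red tower, then checks every Tick whether EXP has reached an age-scaled threshold to age up itself and the tower.
; MeeleTroops, not called here, spawns a BP_ParentTroop at the tower if Money covers MoneySpended, then deducts that troop's TroopCost.
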(event EventBeginPlay
  (bind _returnvalue (Actor|GetActorOfClass "/Game/_Devs/Octavio/BP/GameManager/BP_GameManager.BP_GameManager_C"))
  (Variables|Casts|SetAs%20BP%20Game%20Manager _returnvalue))

(event Collision|EventActorBeginOverlap
  (params (OtherActor :type Actor%20Object%20Reference)))

(event EventTick
  (params (DeltaSeconds :type Float%20%28single-precision%29))
  (CallFunction|CheckifCanAgeUp))

(fn ConstructionScript)

(fn MeeleTroops
  (bind _as_bp_game_manager (Variables|Casts|GetAs%20BP%20Game%20Manager))
  (bind _redteamtower (Variables|/Game/_Devs/Octavio/BP/GameManager/BP_GameManager.BP_GameManager_C|GetRedTeamTower _as_bp_game_manager))
  (if (>= (Variables|PlayerVariables|GetMoney) (Variables|PlayerVariables|GetMoneySpended))
    (bind _returnvalue (Game|SpawnActorfromClass "/Game/_Devs/Octavio/BP/Troops/ParentTroop/BP_ParentTroop.BP_ParentTroop_C" (Math|Transform|MakeTransform (+ (Transformation|GetActorLocation _redteamtower) "0.000000,0.000000,-15.000000") (Transformation|GetActorRotation _redteamtower) "1.000000,1.000000,1.000000") "Undefined" "MultiplyWithRoot" 0 (Variables|/Game/_Devs/Octavio/BP/TowerBase/BP_Tower.BP_Tower_C|GetRedTeamTower? _redteamtower) 0))
    (bind _output_get (Variables|PlayerVariables|SetMoney (- (Variables|PlayerVariables|GetMoney) (Variables|/Game/_Devs/Octavio/BP/Troops/ParentTroop/BP_ParentTroop.BP_ParentTroop_C|GetTroopCost _returnvalue))))
    (Development|PrintString (Utilities|String|ToString(Integer) _output_get))
    (else
      (Development|PrintString "No hay dinero"))))

(fn CheckifCanAgeUp
  (if (>= (Variables|PlayerVariables|GetEXP) (* (Variables|PlayerVariables|GetAI%20CurrentAge) 40))
    (bind _result (Math|Integer|IncrementInt (Variables|PlayerVariables|GetAI%20CurrentAge))
      (:%20%20
        (Variables|PlayerVariables|SetAI%20CurrentAge _result)
        (Default|AgeUp (Variables|/Game/_Devs/Octavio/BP/GameManager/BP_GameManager.BP_GameManager_C|GetRedTeamTower (Variables|Casts|GetAs%20BP%20Game%20Manager)))))))