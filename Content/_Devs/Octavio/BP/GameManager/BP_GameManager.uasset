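; Game manager that holds references to the player and the two team towers and runs the troop training timer.
; On BeginPlay it caches BP_Player, then sorts the first two BP_Tower actors found into red and blue by their team flag.
; TroopSpawnTimer plays a timeline at a rate inverse to RefSpawnTime, counting that same variable down to zero.
; On finish it calls MeeleTroops on the player's widget and clears its training flag.
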(event Custom|TroopSpawnTimer
  (Components|Timeline|SetPlayRate (Variables|Default|GetSpawnTime) (/ 1.0 (Variables|Default|GetRefSpawnTime)))
  (bind _alpha (Timeline|SpawnTime PlayFromStart)
    (:Update
      (Variables|Default|SetRefSpawnTime (Math|Float|Lerp 1.0 0.0 _alpha)))
    (:Finished
      (Default|MeeleTroops (Variables|/Game/_Devs/Octavio/BP/Player/BP_Player.BP_Player_C|GetAs%20WBP%20Player (Variables|Default|GetAs%20BP%20Player)))
      (Variables|/Game/_Devs/Mata/WBP_Player.WBP_Player_C|SetIsTroopTraining? (Variables|/Game/_Devs/Octavio/BP/Player/BP_Player.BP_Player_C|GetAs%20WBP%20Player (Variables|Default|GetAs%20BP%20Player)) false))))

(event EventBeginPlay
  (bind _asbp_player (Utilities|Casting|CastToBP_Player (Game|GetPlayerCharacter 0)))
  (Variables|Default|SetAs%20BP%20Player _asbp_player)
  (CallFunction|GetTowerReference))

(event Collision|EventActorBeginOverlap
  (params (OtherActor :type Actor%20Object%20Reference)))

(event EventTick
  (params (DeltaSeconds :type Float%20%28single-precision%29)))

(fn ConstructionScript)

(fn GetTowerReference
  (bind _outactors (Actor|GetAllActorsOfClass "/Game/_Devs/Octavio/BP/TowerBase/BP_Tower.BP_Tower_C"))
  (Utilities|FlowControl|Sequence
    (:then_0
      (if (Variables|/Game/_Devs/Octavio/BP/TowerBase/BP_Tower.BP_Tower_C|GetRedTeamTower? (Utilities|Array|Get(acopy) _outactors))
        (Variables|Default|SetRedTeamTower (Utilities|Array|Get(acopy) _outactors))
        (else
          (Variables|Default|SetBlueTeamTower (Utilities|Array|Get(acopy) _outactors)))))
    (:then_1
      (if (Variables|/Game/_Devs/Octavio/BP/TowerBase/BP_Tower.BP_Tower_C|GetRedTeamTower? (Utilities|Array|Get(acopy) _outactors 1))
        (Variables|Default|SetRedTeamTower (Utilities|Array|Get(acopy) _outactors 1))
        (else
          (Variables|Default|SetBlueTeamTower (Utilities|Array|Get(acopy) _outactors 1)))))))