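; Base troop for a two-team lane battler that marches along X toward the opposing side, with direction set by team.
; BeginPlay scales health, damage and cost by the player's age, deriving kill rewards and the game manager's spawn time.
; Range and distance overlaps set attack/walk states and halt movement; live logic here never deals damage.
; Death updates player money and EXP for red troops; AI rewards are only a debug print.
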(event Game|Damage|EventAnyDamage
  (params (Damage :type Float%20%28single-precision%29) (DamageType :type Damage%20Type%20Object%20Reference) (InstigatedBy :type Controller%20Object%20Reference) (DamageCauser :type Actor%20Object%20Reference))
  (Variables|InitialStats|SetTroopCurrentHealth (- (Variables|InitialStats|GetTroopCurrentHealth) Damage))
  (CallFunction|DetermineHealth))

(event Collision|EventActorBeginOverlap
  (params (OtherActor :type Actor%20Object%20Reference)))

(event EventTick
  (params (DeltaSeconds :type Float%20%28single-precision%29))
  (Pawn|Input|AddMovementInput (Math|Vector|MakeVector 1.0 0.0 0.0) (Variables|InitialStats|GetMoveScale) false))

(event EventBeginPlay
  (Get|GetPlayerEra)
  (Set|SetTroopCost)
  (Set|SetSpawnTime)
  (Set|SetHealthBar)
  (Set|SetMovementDirection)
  (Set|SetDamage))

(event OnComponentEndOverlap(RangeForAttack)
  (params (OverlappedComponent :type Primitive%20Component%20Object%20Reference) (OtherActor :type Actor%20Object%20Reference) (OtherComp :type Primitive%20Component%20Object%20Reference) (OtherBodyIndex :type Integer))
  (bind _asbp_parent_troop (Utilities|Casting|CastToBP_ParentTroop OtherActor))
  (if (!= (Variables|BP_ParentTroop_C|GetRedTeam? _asbp_parent_troop) (Variables|InitialStats|GetRedTeam?))
    (Variables|AnimationBools|SetIsAttacking false)
    (Variables|AnimationBools|SetIsWalking true)))

(event OnComponentBeginOverlap(RangeForAttack)
  (params (OverlappedComponent :type Primitive%20Component%20Object%20Reference) (OtherActor :type Actor%20Object%20Reference) (OtherComp :type Primitive%20Component%20Object%20Reference) (OtherBodyIndex :type Integer) (bFromSweep :type Boolean) (SweepResult :type Hit%20Result%20Structure%20%28by%20ref%29))
  (bind _asbp_parent_troop (Utilities|Casting|CastToBP_ParentTroop OtherActor)
    (:then
      (Variables|Casts|SetOtherParentTroop _asbp_parent_troop)
      (if (!= (Variables|BP_ParentTroop_C|GetRedTeam? _asbp_parent_troop) (Variables|InitialStats|GetRedTeam?))
        (Variables|AnimationBools|SetIsAttackingTower? false)
        (Variables|AnimationBools|SetIsAttacking true :!label _label)))
    (:CastFailed
      (bind _asbp_tower (Utilities|Casting|CastToBP_Tower OtherActor))
      (bind _output_get (Variables|Casts|SetAs%20BP%20Tower _asbp_tower))
      (if (!= (Variables|/Game/_Devs/Octavio/BP/TowerBase/BP_Tower.BP_Tower_C|GetRedTeamTower? _output_get) (Variables|InitialStats|GetRedTeam?))
        (Variables|AnimationBools|SetIsAttackingTower? true)
        (Variables|InitialStats|SetMoveScale 0.0)
        (goto _label)))))

(event OnComponentBeginOverlap(DistanceChecker)
  (params (OverlappedComponent :type Primitive%20Component%20Object%20Reference) (OtherActor :type Actor%20Object%20Reference) (OtherComp :type Primitive%20Component%20Object%20Reference) (OtherBodyIndex :type Integer) (bFromSweep :type Boolean) (SweepResult :type Hit%20Result%20Structure%20%28by%20ref%29))
  (Utilities|Casting|CastToBP_ParentTroop OtherActor)
  (Variables|InitialStats|SetMoveScale 0.0)
  (if (not (Variables|AnimationBools|GetIsAttacking))
    (Variables|AnimationBools|SetIsAttacking false)
    (Variables|AnimationBools|SetIsWalking false)))

(event OnComponentEndOverlap(DistanceChecker)
  (params (OverlappedComponent :type Primitive%20Component%20Object%20Reference) (OtherActor :type Actor%20Object%20Reference) (OtherComp :type Primitive%20Component%20Object%20Reference) (OtherBodyIndex :type Integer))
  (Utilities|Casting|CastToBP_ParentTroop OtherActor)
  (Variables|AnimationBools|SetIsAttacking false)
  (Set|SetMovementDirection))

(fn ConstructionScript)

(fn SetMovementDirection
  (Variables|AnimationBools|SetIsWalking true)
  (if (Variables|InitialStats|GetRedTeam?)
    (Variables|InitialStats|SetMoveScale -0.06)
    (Transformation|SetActorRotation "0.000000,180.000000,0.000000")
    (else
      (Variables|InitialStats|SetMoveScale 0.06))))

(fn GetPlayerEra
  (bind _asbp_player (Utilities|Casting|CastToBP_Player (Game|GetPlayerCharacter 0)))
  (Variables|Casts|SetAs%20BP%20Player _asbp_player)
  (bind _returnvalue (Actor|GetActorOfClass "/Game/_Devs/Octavio/BP/GameManager/BP_GameManager.BP_GameManager_C"))
  (Variables|Casts|SetAs%20BP%20GameManager _returnvalue))

(fn SetHealthBar
  (Variables|ChildVariables|SetTroopMaxHealth (* (Variables|/Game/_Devs/Octavio/BP/Player/BP_Player.BP_Player_C|GetPlayerCurrentAge (Variables|Casts|GetAs%20BP%20Player)) (Variables|ChildVariables|GetTroopMaxHealth)))
  (bind _aswbp_troop_health (Utilities|Casting|CastToWBP_TroopHealth (UserInterface|GetUserWidgetObject (Variables|Default|GetHealthBar))))
  (bind _output_get (Variables|Casts|SetAs%20WBP%20Troop%20Health _aswbp_troop_health))
  (bind _output_get_2 (Variables|/Game/_Devs/Octavio/BP/Widgets/Troops/WBP_TroopHealth.WBP_TroopHealth_C|SetMaxHealth _output_get (Variables|ChildVariables|GetTroopMaxHealth)))
  (Variables|InitialStats|SetTroopCurrentHealth _output_get_2))

(fn DetermineHealth
  (Variables|/Game/_Devs/Octavio/BP/Widgets/Troops/WBP_TroopHealth.WBP_TroopHealth_C|SetCurrentHealth (Variables|Casts|GetAs%20WBP%20Troop%20Health) (Variables|InitialStats|GetTroopCurrentHealth))
  (if (<= (Variables|InitialStats|GetTroopCurrentHealth) 0.0)
    (CallFunction|DetermineGivenMoney&EXP)
    (Actor|DestroyActor)))

(fn SetDamage
  (Variables|ChildVariables|SetDamage (* (Variables|/Game/_Devs/Octavio/BP/Player/BP_Player.BP_Player_C|GetPlayerCurrentAge (Variables|Casts|GetAs%20BP%20Player)) (Variables|ChildVariables|GetDamage))))

(fn SetTroopCost
  (bind _output_get (Variables|ChildVariables|SetTroopCost (* (Variables|ChildVariables|GetTroopCost) (Variables|/Game/_Devs/Octavio/BP/Player/BP_Player.BP_Player_C|GetPlayerCurrentAge (Variables|Casts|GetAs%20BP%20Player)))))
  (bind _output_get_2 (Variables|InitialStats|SetGivenMoney (Math|Float|Ceil (* _output_get 1.3))))
  (Variables|InitialStats|SetGivenExp (* _output_get_2 2)))

(fn DetermineGivenMoney&EXP
  (bind _as_bp_player (Variables|Casts|GetAs%20BP%20Player))
  (if (Variables|InitialStats|GetRedTeam?)
    (Variables|/Game/_Devs/Octavio/BP/Player/BP_Player.BP_Player_C|SetMoney _as_bp_player (+ (Variables|/Game/_Devs/Octavio/BP/Player/BP_Player.BP_Player_C|GetMoney _as_bp_player) (Variables|InitialStats|GetGivenMoney)))
    (Variables|/Game/_Devs/Octavio/BP/Player/BP_Player.BP_Player_C|SetEXP _as_bp_player (+ (Variables|/Game/_Devs/Octavio/BP/Player/BP_Player.BP_Player_C|GetEXP _as_bp_player) (Variables|InitialStats|GetGivenExp)))
    (Default|DeterminePlayerEconomy&EXP _as_bp_player)
    (Default|CheckifCanAgeUp _as_bp_player)
    (else
      (Development|PrintString "Give Money and EXP to AI"))))

(fn SetSpawnTime
  (bind _output_get (Variables|ChildVariables|SetSpawnTime (/ (/ (Variables|InitialStats|GetGivenMoney) 2) 10)))
  (Variables|/Game/_Devs/Octavio/BP/GameManager/BP_GameManager.BP_GameManager_C|SetRefSpawnTime (Variables|Casts|GetAs%20BP%20GameManager) _output_get))