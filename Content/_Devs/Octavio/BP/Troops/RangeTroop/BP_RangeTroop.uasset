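; Ranged troop Blueprint, a child troop class that sets its own health, damage and cost.
; BeginPlay applies these values before running the parent's BeginPlay, then selects the troop's animation instance class.
; SetTroopSprite reads the current age from the AI pawn for the red team, otherwise from the player, mapping the first age to the parent troop animation and the next to a range-specific one.
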(event EventBeginPlay
  (CallFunction|SetChildValues)
  (|CallParentFunction)
  (CallFunction|SetTroopSprite))

(event Collision|EventActorBeginOverlap
  (params (OtherActor :type Actor%20Object%20Reference))
  (|CallParentFunction OtherActor) ; This node is disabled and will not be called.\nDrag off pins to build functionality.
)

(event EventTick
  (params (DeltaSeconds :type Float%20%28single-precision%29))
  (|CallParentFunction DeltaSeconds) ; This node is disabled and will not be called.\nDrag off pins to build functionality.
)

(fn ConstructionScript
  (|CallParentFunction))

(fn SetTroopSprite
  (bind _animationcomponent (Variables|Default|GetAnimationComponent))
  (bind _animationcomponent_2 (Variables|Default|GetAnimationComponent))
  (if (Variables|Default|GetRedTeam?)
    (switch int (Variables|/Game/_Devs/Octavio/BP/IA/BP_IAPawn.BP_IAPawn_C|GetAI%20CurrentAge (Variables|Default|GetAs%20BP%20AIPawn))
      (:0
        (Class|PaperZDAnimationComponent|SetAnimInstanceClass _animationcomponent_2 "/Game/_Devs/Octavio/BP/Troops/_ParentTroop/ABP_ParentTroop.ABP_ParentTroop_C"))
      (:1
        (Class|PaperZDAnimationComponent|SetAnimInstanceClass _animationcomponent_2 "/Game/_Devs/Octavio/BP/Troops/RangeTroop/1EraAnim/ABP_1Era_Range.ABP_1Era_Range_C")))
    (else
      (switch int (Variables|/Game/_Devs/Octavio/BP/Player/BP_Player.BP_Player_C|GetPlayerCurrentAge (Variables|Default|GetAs%20BP%20Player))
        (:0
          (Class|PaperZDAnimationComponent|SetAnimInstanceClass _animationcomponent "/Game/_Devs/Octavio/BP/Troops/_ParentTroop/ABP_ParentTroop.ABP_ParentTroop_C"))
        (:1
          (Class|PaperZDAnimationComponent|SetAnimInstanceClass _animationcomponent "/Game/_Devs/Octavio/BP/Troops/RangeTroop/1EraAnim/ABP_1Era_Range.ABP_1Era_Range_C"))))))

(fn SetChildValues
  (Variables|Default|SetTroopMaxHealth 75.0)
  (Variables|Default|SetDamage 3e+01)
  (Variables|Default|SetTroopCost 25))