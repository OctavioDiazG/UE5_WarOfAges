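; BP_Tower is the base tower for either the player or AI team, ending the game when destroyed.
; On BeginPlay it scales max health by the owning side's age, feeds its health bar widget and spawns two team troops 20 seconds apart.
; Damage updates health; at zero it prints the result and pauses.
; AgeUp recolors sprite instances and refills health, compounding the age multiplier on current max.
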(event EventBeginPlay
  (bind _asbp_player (Utilities|Casting|CastToBP_Player (Game|GetPlayerCharacter 0)))
  (Variables|Casts|SetAs%20BP%20Player _asbp_player)
  (bind _aswbp_tower_health (Utilities|Casting|CastToWBP_TowerHealth (UserInterface|GetUserWidgetObject (Variables|Default|GetHealthBar))))
  (Variables|Casts|SetAs%20WBP%20Tower%20Health _aswbp_tower_health)
  (bind _returnvalue (Actor|GetActorOfClass "/Game/_Devs/Octavio/BP/IA/BP_IAPawn.BP_IAPawn_C"))
  (Variables|Casts|SetAs%20BP%20AIPawn _returnvalue)
  (CallFunction|SetHealth)
  (Game|SpawnActorfromClass "/Game/_Devs/Octavio/BP/Troops/ParentTroop/BP_ParentTroop.BP_ParentTroop_C" (Math|Transform|MakeTransform (+ (.location (Transformation|GetActorTransform)) (Math|Vector|MakeVector (.x (Transformation|GetActorForwardVector)) 0.0 -15.0)) "0, 0, 0" "1.000000,1.000000,1.000000") "Undefined" "MultiplyWithRoot" 0 (Variables|Default|GetRedTeamTower?) 0)
  (Utilities|FlowControl|Delay 2e+01)
  (Game|SpawnActorfromClass "/Game/_Devs/Octavio/BP/Troops/ParentTroop/BP_ParentTroop.BP_ParentTroop_C" (Math|Transform|MakeTransform (+ (.location (Transformation|GetActorTransform)) (Math|Vector|MakeVector (.x (Transformation|GetActorForwardVector)) 0.0 -15.0)) "0, 0, 0" "1.000000,1.000000,1.000000") "Undefined" "MultiplyWithRoot" 0 (Variables|Default|GetRedTeamTower?) 0))

(event Collision|EventActorBeginOverlap
  (params (OtherActor :type Actor%20Object%20Reference)))

(event EventTick
  (params (DeltaSeconds :type Float%20%28single-precision%29)))

(event Game|Damage|EventAnyDamage
  (params (Damage :type Float%20%28single-precision%29) (DamageType :type Damage%20Type%20Object%20Reference) (InstigatedBy :type Controller%20Object%20Reference) (DamageCauser :type Actor%20Object%20Reference))
  (Variables|Default|SetTowerCurrentHealth (- (Variables|Default|GetTowerCurrentHealth) Damage))
  (CallFunction|DetermineHealth))

(fn ConstructionScript)

(fn SetHealth
  (if (Variables|Default|GetRedTeamTower?)
    ;[1 1 1] AI Base
    (bind _output_get (Variables|Default|SetTowerMaxHealth (* (Variables|/Game/_Devs/Octavio/BP/IA/BP_IAPawn.BP_IAPawn_C|GetAI%20CurrentAge (Variables|Casts|GetAs%20BP%20AIPawn)) (Variables|Default|GetTowerMaxHealth))))
    (bind _output_get_2 (Variables|/Game/_Devs/Octavio/BP/Widgets/Tower/WBP_TowerHealth.WBP_TowerHealth_C|SetMaxHealth (Variables|Casts|GetAs%20WBP%20Tower%20Health) _output_get))
    (Variables|Default|SetTowerCurrentHealth _output_get_2)
    (CallFunction|DetermineHealth)
    (else
      ;[1 1 1] Player Base
      (bind _output_get_3 (Variables|Default|SetTowerMaxHealth (* (Variables|/Game/_Devs/Octavio/BP/Player/BP_Player.BP_Player_C|GetPlayerCurrentAge (Variables|Casts|GetAs%20BP%20Player)) (Variables|Default|GetTowerMaxHealth))))
      (bind _output_get_4 (Variables|/Game/_Devs/Octavio/BP/Widgets/Tower/WBP_TowerHealth.WBP_TowerHealth_C|SetMaxHealth (Variables|Casts|GetAs%20WBP%20Tower%20Health) _output_get_3))
      (Variables|Default|SetTowerCurrentHealth _output_get_4)
      (CallFunction|DetermineHealth))))

(fn DetermineHealth
  (Variables|/Game/_Devs/Octavio/BP/Widgets/Tower/WBP_TowerHealth.WBP_TowerHealth_C|SetCurrentHealth (Variables|Casts|GetAs%20WBP%20Tower%20Health) (Variables|Default|GetTowerCurrentHealth))
  (if (<= (Variables|Default|GetTowerCurrentHealth) 0.0)
    (CallFunction|DetermineWinner)))

(fn DetermineWinner
  (if (Variables|Default|GetRedTeamTower?)
    (Development|PrintString "Finish Game YouWon")
    (else
      (Development|PrintString "Finish Game YouLoss")))
  (Game|SetGamePaused true))

(fn AgeUp
  (bind _papergroupedsprite (Variables|Default|GetPaperGroupedSprite))
  (bind _towercurrenthealth (Variables|Default|GetTowerCurrentHealth))
  (bind _towermaxhealth (Variables|Default|GetTowerMaxHealth))
  (bind _returnvalue (+ _towercurrenthealth _towermaxhealth))
  (bind _returnvalue_2 (/ _returnvalue 1e+03))
  (Class|PaperGroupedSpriteComponent|UpdateInstanceColor _papergroupedsprite 0 (Utilities|Struct|MakeLinearColor 0.0 _returnvalue_2 0.0 1.0) true)
  (Class|PaperGroupedSpriteComponent|UpdateInstanceColor _papergroupedsprite 1 (Utilities|Struct|MakeLinearColor 0.0 _returnvalue_2 0.0 1.0) true)
  (CallFunction|SetHealth))