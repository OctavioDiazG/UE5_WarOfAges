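; Player pawn that holds money, veterancy EXP and current age, and shows them through a WBP_Player HUD.
; On BeginPlay it creates the widget, pushes Money and EXP to it, sets the age to 1 and registers the default Enhanced Input mapping.
; Movement input only drives along the forward vector.
; CheckIfCanAgeUp, not called here, enables the Age Up button once EXP reaches a threshold scaled by current age.
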(event Input|EnhancedActionEvents|EnhancedInputActionIA_Movement
  (params (ActionValue :type Float%20%28double-precision%29) (ElapsedSeconds :type Float%20%28double-precision%29) (TriggeredSeconds :type Float%20%28double-precision%29) (InputAction :type Input%20Action%20Object%20Reference :default "/Game/_Devs/Octavio/BP/Player/IA_Movement.IA_Movement"))
  (:Triggered
    (Pawn|Input|AddMovementInput (Transformation|GetActorForwardVector) ActionValue false)))

(event EventBeginPlay
  (bind _returnvalue (UserInterface|CreateWidget "/Game/_Devs/Mata/WBP_Player.WBP_Player_C"))
  (bind _output_get (Variables|Casts|SetAs%20WBP%20Player _returnvalue))
  (UserInterface|Viewport|AddtoViewport _output_get 0)
  (CallFunction|DetermineEconomy)
  (CallFunction|DetermineEXPVeterancy)
  (Variables|Default|SetPlayerCurrentAge 1)
  (bind _asplayer_controller (Utilities|Casting|CastToPlayerController (Pawn|GetController)))
  (Input|AddMappingContext (PlayerController|LocalPlayerSubsystems|GetEnhancedInputLocalPlayerSubsystem _asplayer_controller) "/Game/_Devs/Octavio/BP/Player/IMC_Default.IMC_Default" 0 "(bIgnoreAllPressedKeysUntilRelease=True,bForceImmediately=False)"))

(fn ConstructionScript)

(fn CheckifCanAgeUp
  (bind _as_wbp_player (Variables|Casts|GetAs%20WBP%20Player))
  (bind _ageup (Variables|/Game/_Devs/Mata/WBP_Player.WBP_Player_C|GetAgeUp _as_wbp_player))
  (if (>= (Variables|Default|GetEXP) (* (Variables|Default|GetPlayerCurrentAge) 40))
    (Variables|/Script/UMG.Widget|SetbIsEnabled _ageup true)
    (else
      (Variables|/Script/UMG.Widget|SetbIsEnabled _ageup false))))

(fn DetermineEconomy
  (bind _output_get (Variables|Default|SetMoney (Variables|Default|GetMoney)))
  (Variables|/Game/_Devs/Mata/WBP_Player.WBP_Player_C|SetCurrency (Variables|Casts|GetAs%20WBP%20Player) _output_get))

(fn DetermineEXPVeterancy
  (bind _output_get (Variables|Default|SetEXP (Variables|Default|GetEXP)))
  (Variables|/Game/_Devs/Mata/WBP_Player.WBP_Player_C|SetVeterany (Variables|Casts|GetAs%20WBP%20Player) _output_get))